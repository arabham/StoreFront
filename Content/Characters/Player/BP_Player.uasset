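; BP_Player is the player Blueprint that tracks the player's money and the current day.
; TotalMoney settles the balance by subtracting Losses from Money and adding Sales.
; IncrementDay advances the Day counter by one.
; The construction script is empty, and neither function resets the Sales or Losses totals.
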(fn `IncrementDay`
  (set `self.Day` (+ (`self.Day`) 1))
  (return))

(fn `Total Money`
  (set `self.Money` (+ (- (`self.Money`) (`self.Losses`)) (`self.Sales`)))
  (return))

(fn `UserConstructionScript`)